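; Decal actor that displays a number of up to four digits with an m or km unit, built from font decals.
; The construction script toggles the unit decals from Km and can hide leading zeros.
; It pads Number to four digits as text, then maps each character through NumberToDecal to a font material for its decal.
; UpdateDecals duplicates this logic as an event, but never re-shows hidden digits.
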(event Custom|UpdateDecals
  (bind _km (Variables|Default|Getkm))
  (bind _number (Variables|Default|GetNumber))
  (bind _number_2 (Variables|Default|GetNumber))
  (bind _returnvalue (Utilities|Text|ToText(Integer) _number false false 4 4))
  (bind _returnvalue_2 (Utilities|String|ToString(Text) _returnvalue))
  (Utilities|FlowControl|Sequence
    (:then_0
      (Rendering|SetVisibility (Variables|Default|Getk) _km false)
      (Rendering|SetVisibility (Variables|Default|Getm1) _km false)
      (Rendering|SetVisibility (Variables|Default|Getm0) (not _km) false)
      (if (Variables|Default|GetCutoffLeadingZeros)
        (if (< _number_2 1000)
          (Rendering|SetVisibility (Variables|Default|Get3) false false))
        (if (< _number_2 100)
          (Rendering|SetVisibility (Variables|Default|Get2) false false))
        (if (< _number_2 10)
          (Rendering|SetVisibility (Variables|Default|Get1) false false))))
    (:then_1
      (bind _decal (CallFunction|NumbertoDecal (Math|Conversions|ToInteger(Byte) (Utilities|String|GetSubstring _returnvalue_2 3))))
      (Rendering|Components|Decal|SetDecalMaterial (Variables|Default|Get0) _decal)
      (bind _decal_2 (CallFunction|NumbertoDecal (Math|Conversions|ToInteger(Byte) (Utilities|String|GetSubstring _returnvalue_2 2))))
      (Rendering|Components|Decal|SetDecalMaterial (Variables|Default|Get1) _decal_2)
      (bind _decal_3 (CallFunction|NumbertoDecal (Math|Conversions|ToInteger(Byte) (Utilities|String|GetSubstring _returnvalue_2 1))))
      (Rendering|Components|Decal|SetDecalMaterial (Variables|Default|Get2) _decal_3)
      (bind _decal_4 (CallFunction|NumbertoDecal (Math|Conversions|ToInteger(Byte) (Utilities|String|GetSubstring _returnvalue_2 0))))
      (Rendering|Components|Decal|SetDecalMaterial (Variables|Default|Get3) _decal_4))))

(event EventBeginPlay)

(event Collision|EventActorBeginOverlap
  (params (OtherActor :type Actor%20Object%20Reference)))

(event EventTick
  (params (DeltaSeconds :type Float%20%28single-precision%29)))

(fn ConstructionScript
  (bind _km (Variables|Default|Getkm))
  (bind _number (Variables|Default|GetNumber))
  (bind _number_2 (Variables|Default|GetNumber))
  (bind _returnvalue (Utilities|Text|ToText(Integer) _number false false 4 4))
  (bind _returnvalue_2 (Utilities|String|ToString(Text) _returnvalue))
  (Utilities|FlowControl|Sequence
    (:then_0
      (Rendering|SetVisibility (Variables|Default|Getk) _km false)
      (Rendering|SetVisibility (Variables|Default|Getm1) _km false)
      (Rendering|SetVisibility (Variables|Default|Getm0) (not _km) false)
      (if (Variables|Default|GetCutoffLeadingZeros)
        (if (< _number_2 1000)
          (Rendering|SetVisibility (Variables|Default|Get3) false false))
        (if (< _number_2 100)
          (Rendering|SetVisibility (Variables|Default|Get2) false false))
        (if (< _number_2 10)
          (Rendering|SetVisibility (Variables|Default|Get1) false false))))
    (:then_1
      (bind _decal (CallFunction|NumbertoDecal (Math|Conversions|ToInteger(Byte) (Utilities|String|GetSubstring _returnvalue_2 3))))
      (Rendering|Components|Decal|SetDecalMaterial (Variables|Default|Get0) _decal)
      (bind _decal_2 (CallFunction|NumbertoDecal (Math|Conversions|ToInteger(Byte) (Utilities|String|GetSubstring _returnvalue_2 2))))
      (Rendering|Components|Decal|SetDecalMaterial (Variables|Default|Get1) _decal_2)
      (bind _decal_3 (CallFunction|NumbertoDecal (Math|Conversions|ToInteger(Byte) (Utilities|String|GetSubstring _returnvalue_2 1))))
      (Rendering|Components|Decal|SetDecalMaterial (Variables|Default|Get2) _decal_3)
      (bind _decal_4 (CallFunction|NumbertoDecal (Math|Conversions|ToInteger(Byte) (Utilities|String|GetSubstring _returnvalue_2 0))))
      (Rendering|Components|Decal|SetDecalMaterial (Variables|Default|Get3) _decal_4))))

(fn NumbertoDecal
  (params (Digit :type Integer))
  (return (Utilities|Select :Index Digit :Option%200 "/EG4U/Roads/Materials/Fontset/font_0.font_0" :Option%201 "/EG4U/Roads/Materials/Fontset/font_1.font_1" :Option%202 "/EG4U/Roads/Materials/Fontset/font_2.font_2" :Option%203 "/EG4U/Roads/Materials/Fontset/font_3.font_3" :Option%204 "/EG4U/Roads/Materials/Fontset/font_4.font_4" :Option%205 "/EG4U/Roads/Materials/Fontset/font_5.font_5" :Option%206 "/EG4U/Roads/Materials/Fontset/font_6.font_6" :Option%207 "/EG4U/Roads/Materials/Fontset/font_7.font_7" :Option%208 "/EG4U/Roads/Materials/Fontset/font_8.font_8" :Option%209 "/EG4U/Roads/Materials/Fontset/font_9.font_9")))