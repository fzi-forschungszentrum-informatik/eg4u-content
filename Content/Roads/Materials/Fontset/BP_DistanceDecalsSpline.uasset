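; Spline actor that places numbered BP_FontDecal distance markers at regular intervals along a road or path.
; SpawnAlongSpline steps along the spline by Interval in meters, spawning and attaching decals that receive their distance, Km and leading-zero settings before updating.
; RemoveDecals destroys the tracked decals and every other attached actor.
; The construction script is empty, with its calls to both events disconnected, so nothing in this Blueprint triggers them.
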(event Custom|SpawnAlongSpline
  (bind _interval (Variables|Default|GetInterval))
  (bind _returnvalue (* _interval 100))
  (bind _returnvalue_2 (Math|Conversions|ToFloat(Integer) _returnvalue))
  (for _index (range 0 (Math|Float|Floor (/ (Spline|GetSplineLength (Variables|Default|GetSpline)) _returnvalue_2)))
    (bind _returnvalue_3 (Game|SpawnActorfromClass "/EG4U/Roads/Materials/Fontset/BP_FontDecal.BP_FontDecal_C" (Math|Transform|MakeTransform (.location (Spline|GetTransformatDistanceAlongSpline (Variables|Default|GetSpline) (* _index _returnvalue_2) "Local" false)) (.rotation (Spline|GetTransformatDistanceAlongSpline (Variables|Default|GetSpline) (* _index _returnvalue_2) "Local" false)) "1,1,1") "AlwaysSpawn" 0 0))
    (Variables|/EG4U/Roads/Materials/Fontset/BP_FontDecal.BP_FontDecal_C|Setkm _returnvalue_3 (Variables|Default|GetKm))
    (Variables|/EG4U/Roads/Materials/Fontset/BP_FontDecal.BP_FontDecal_C|SetCutoffLeadingZeros _returnvalue_3 (Variables|Default|GetCutoff%20Leading%20Zeros))
    (Variables|/EG4U/Roads/Materials/Fontset/BP_FontDecal.BP_FontDecal_C|SetNumber _returnvalue_3 (/ (* _index _returnvalue) 100))
    (Default|UpdateDecals _returnvalue_3)
    (Utilities|Array|Add (Variables|Default|GetDecals) _returnvalue_3)
    (Transformation|AttachActorToActor _returnvalue_3 self "None" "KeepRelative" "KeepRelative" "KeepRelative" true)))

(event Custom|RemoveDecals
  (bind _decals (Variables|Default|GetDecals))
  (for _array_element _decals
    (Actor|DestroyActor _array_element))
  (Utilities|Array|Clear _decals)
  (for _array_element_2 (Actor|GetAttachedActors false)
    (Actor|DestroyActor _array_element_2)))

(event EventBeginPlay)

(event Collision|EventActorBeginOverlap
  (params (OtherActor :type Actor%20Object%20Reference)))

(event EventTick
  (params (DeltaSeconds :type Float%20%28single-precision%29)))

(fn ConstructionScript)