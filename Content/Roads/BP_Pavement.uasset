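; BP_Pavement is a road pavement actor that can spawn BP_ParkingSpot actors along its spline.
; AddParkedParkingSpots steps along the spline until near its end, placing each spot at a lateral offset in world space.
; A parallel flag selects spots aligned with the spline or turned 90 degrees, with matching spacing, and a forward flag can flip them 180 degrees.
; The event graph and construction script add no logic of their own.
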(event EventBeginPlay
  (|CallParentFunction) ; This node is disabled and will not be called.\nDrag off pins to build functionality.
)

(event Collision|EventActorBeginOverlap
  (params (OtherActor :type Actor%20Object%20Reference)))

(event EventTick
  (params (DeltaSeconds :type Float%20%28single-precision%29)))

(fn ConstructionScript
  (|CallParentFunction))

(fn AddParkedParkingSpots
  (params (InParallel :type Boolean) (Offset :type Float%20%28single-precision%29) (Forward :type Boolean))
  (bind _parallel (Variables|Default|GetParallel))
  (while (< (Variables|Default|GetCurrentLength) (- (Spline|GetSplineLength (Variables|Default|GetSpline)) 5.0))
    (Game|SpawnActorfromClass "/EG4U/Roads/BP_ParkingSpot.BP_ParkingSpot_C" (Math|Transform|MakeTransform (Math|Transform|TransformLocation (Spline|GetTransformatDistanceAlongSpline (Variables|Default|GetSpline) (Variables|Default|GetCurrentLength) "World" false) (Math|Vector|MakeVector 0.0 Offset 0.0)) (Math|Rotator|MakeRotator 0.0 0.0 (+ (Math|Float|SelectFloat (.yaw (.Rotation (Math|Transform|BreakTransform (Spline|GetTransformatDistanceAlongSpline (Variables|Default|GetSpline) (Variables|Default|GetCurrentLength) "World" false)))) (+ (.yaw (.Rotation (Math|Transform|BreakTransform (Spline|GetTransformatDistanceAlongSpline (Variables|Default|GetSpline) (Variables|Default|GetCurrentLength) "World" false)))) 9e+01) _parallel) (Math|Float|SelectFloat 0.0 1.8e+02 Forward))) "1,1,1") "Undefined" 0 0)
    (Variables|Default|SetCurrentLength (+ (Math|Float|SelectFloat 5.5e+02 2.8e+02 _parallel) (Variables|Default|GetCurrentLength)))))