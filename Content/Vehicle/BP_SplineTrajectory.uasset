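; BP_SplineTrajectory is a spline path actor that hands its route to AI-driven vehicles entering its trigger box.
; On overlap, it pauses the OpenDRIVE_RoadControl controller's PID steering, then after a short delay resets it, assigns the spline and resumes.
; Helper functions build the spline from scaled, optionally reversed points, snap its ends to Successor and Predecessor last points, and move the box to the spline start.
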(event OnComponentBeginOverlap(Box)
  (params (OverlappedComponent :type Primitive%20Component%20Object%20Reference) (OtherActor :type Actor%20Object%20Reference) (OtherComp :type Primitive%20Component%20Object%20Reference) (OtherBodyIndex :type Integer) (bFromSweep :type Boolean) (SweepResult :type Hit%20Result%20Structure%20%28by%20ref%29))
  (bind _aswheeled_vehicle (Utilities|Casting|CastToWheeledVehicle OtherActor))
  (bind _asopen_drive_road_control (Utilities|Casting|CastToOpenDRIVE_RoadControl (AI|GetAIController _aswheeled_vehicle)))
  (Variables|/EG4U/Vehicle/OpenDRIVE_RoadControl.OpenDRIVE_RoadControl_C|SetPausePID_S _asopen_drive_road_control true)
  (Variables|/Script/EG4U.AI_PIDController|Setcurrent_steering _asopen_drive_road_control 0.0)
  (Utilities|FlowControl|Delay 1.0)
  (Class|AIPIDController|PIDReset _asopen_drive_road_control (Variables|/Script/EG4U.AI_PIDController|Getsteering_gain _asopen_drive_road_control) 0.0 0.0)
  (Variables|/EG4U/Vehicle/OpenDRIVE_RoadControl.OpenDRIVE_RoadControl_C|SetTrajectory _asopen_drive_road_control (Variables|Default|GetSpline))
  (Variables|/EG4U/Vehicle/OpenDRIVE_RoadControl.OpenDRIVE_RoadControl_C|SetPausePID_S _asopen_drive_road_control false))

(event EventBeginPlay)

(event Collision|EventActorBeginOverlap
  (params (OtherActor :type Actor%20Object%20Reference)))

(event EventTick
  (params (DeltaSeconds :type Float%20%28single-precision%29)))

(fn ConstructionScript)

(fn ConnectFollowing
  (bind _predecessor (Variables|Default|GetPredecessor))
  (bind _successor (Variables|Default|GetSuccessor))
  (bind _spline (Variables|Default|GetSpline))
  (bind _returnvalue (Spline|GetNumberOfSplinePoints _spline))
  (bind _spline_2 (Variables|BP_SplineTrajectory_C|GetSpline _predecessor))
  (bind _spline_3 (Variables|BP_SplineTrajectory_C|GetSpline _successor))
  (bind _returnvalue_2 (- _returnvalue 1))
  (bind _returnvalue_3 (Spline|GetNumberOfSplinePoints _spline_3))
  (bind _returnvalue_4 (Spline|GetNumberOfSplinePoints _spline_2))
  (bind _returnvalue_5 (- _returnvalue_3 1))
  (bind _returnvalue_6 (- _returnvalue_4 1))
  (bind (_location _tangent) (Spline|GetLocationandTangentatSplinePoint _spline_2 _returnvalue_6 "World"))
  (bind (_location_2 _tangent_2) (Spline|GetLocationandTangentatSplinePoint _spline_3 _returnvalue_5 "World"))
  (Utilities|FlowControl|Sequence
    (:then_0
      (if (Utilities|IsValid _successor)
        (Spline|SetLocationatSplinePoint (Variables|Default|GetSpline) _returnvalue_2 _location_2 "World" true)
        (Spline|SetTangentatSplinePoint (Variables|Default|GetSpline) _returnvalue_2 _tangent_2 "World" true)))
    (:then_1
      (if (Utilities|IsValid _predecessor)
        (Spline|SetLocationatSplinePoint (Variables|Default|GetSpline) 0 _location "World" true)
        (Spline|SetTangentatSplinePoint (Variables|Default|GetSpline) 0 _tangent "World" true)))))

(fn SetPoints
  (params (InPoints :type Array%20of%20Vectors) (Scale :type Vector) (Reverse :type Boolean))
  (bind _output_get (Variables|Default|SetSampledPoints InPoints))
  (if Reverse
    (Utilities|Array|Reverse _output_get))
  (CallFunction|ScalePoints Scale)
  (Spline|ClearSplinePoints (Variables|Default|GetSpline) true)
  (Spline|SetSplinePoints (Variables|Default|GetSpline) _output_get "Local" true))

(fn ScalePoints
  (params (Scale :type Vector))
  (bind _sampledpoints (Variables|Default|GetSampledPoints))
  (for (_array_element _array_index) _sampledpoints
    (Utilities|Array|SetArrayElem _sampledpoints _array_index (* _array_element Scale))))

(fn UpdateBox
  (bind _spline (Variables|Default|GetSpline))
  (bind (_location _tangent) (Spline|GetLocationandTangentatSplinePoint _spline 0 "World"))
  (Transformation|SetWorldLocationAndRotation (Variables|Default|GetBox) _location (Math|Rotator|MakeRotator 0.0 0.0 (.z _tangent)) false false))